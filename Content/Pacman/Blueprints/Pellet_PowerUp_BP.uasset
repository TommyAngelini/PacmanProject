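; Power-up pellet Blueprint for the Pac-Man game that reacts to pellet-eaten events.
; On BeginPlay it binds a handler that calls ApplyPowerUpMovement on the player's Pacman pawn when the pellet type is PowerUp.
; The handler also decrements the game mode's remaining pellet count for any type.
; When that count reaches zero, it sets GameWon and plays the victory sound.
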(event Custom|On%20Pellet%20Eaten%20Event
  (params (PelletType :type EPelletType%20Enum :default "Regular"))
  (Utilities|FlowControl|Sequence
    (:then_0
      (if (Utilities|Enum|Equal(Enum) PelletType "PowerUp")
        (bind _aspacman_bp (Utilities|Casting|CastToPacman_BP (Game|Player|GetPlayerPawn 0)))
        (Default|ApplyPowerUpMovement _aspacman_bp)))
    (:then_1
      (bind _aspacman_game_mode_bp (Utilities|Casting|CastToPacman_GameMode_BP (Game|GetGameMode)))
      (bind _output_get (Variables|/Game/Pacman/Blueprints/Pacman_GameMode_BP.Pacman_GameMode_BP_C|SetNumPelletsLeft _aspacman_game_mode_bp (- (Variables|/Game/Pacman/Blueprints/Pacman_GameMode_BP.Pacman_GameMode_BP_C|GetNumPelletsLeft _aspacman_game_mode_bp) 1.0)))
      (if (== _output_get 0.0)
        (bind _aspacman_game_mode_bp_2 (Utilities|Casting|CastToPacman_GameMode_BP (Game|GetGameMode)))
        (Variables|/Game/Pacman/Blueprints/Pacman_GameMode_BP.Pacman_GameMode_BP_C|SetGameWon _aspacman_game_mode_bp_2 true)
        (Audio|PlaySound2D "/Game/Pacman/Audio/AM_GameEndedVictoryCue.AM_GameEndedVictoryCue" 1.0 1.0 0.0 0 0)))))

(event EventBeginPlay
  (EventDispatchers|BindEventtoPelletEatenEvent (delegate Custom|On%20Pellet%20Eaten%20Event)))

(fn ConstructionScript)