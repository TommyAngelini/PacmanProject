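; Game mode for a Pac-Man style game that starts a round when play begins.
; BeginPlay resets the win flag, sets a fixed pellet count, plays a gameplay audio cue and marks the game live.
; It also blends the player view to the first CameraActor found in the level, then unfreezes the Pac-Man pawn after a short delay.
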(event Custom|Setup%20Camera
  (bind _outactors (Actor|GetAllActorsOfClass "/Script/Engine.CameraActor"))
  (Game|Player|SetViewTargetwithBlend (Game|GetPlayerController 0) (Utilities|Array|Get(acopy) _outactors) 1.0 "VTBlend_Linear" 0.0 false))

(event EventBeginPlay
  (Utilities|FlowControl|Sequence
    (:then_0
      (Variables|Default|SetGameWon false))
    (:then_1
      (Variables|Default|SetNumPelletsLeft 198.0))
    (:then_2
      (CallFunction|SetupCamera)
      (Utilities|FlowControl|Delay 2.0)
      (bind _aspacman_bp (Utilities|Casting|CastToPacman_BP (Game|Player|GetPlayerPawn 0)))
      (Class|PacmanPawn|SetFrozen _aspacman_bp false))
    (:then_3
      (Audio|PlaySound2D "/Game/Pacman/Audio/AM_GameplayCue.AM_GameplayCue" 1.0 1.0 0.0 0 0))
    (:then_4
      (Variables|Default|SetGameLive true))))

(fn ConstructionScript)